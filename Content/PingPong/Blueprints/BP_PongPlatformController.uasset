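; Player controller for networked Pong that relays paddle movement and ball respawn requests.
; ServerMoveVertical passes a delta to MulticastMoveVertical, which moves the controlled BP_PlatformPawn, but the MoveVertical axis input is empty and its movement calculation is disconnected.
; The RespawnBall input calls ServerRespawnBall, which destroys the game mode's Ball; no spawning happens here.
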(event `self.ReceiveBeginPlay`)

(event `InputAxis|MoveVertical`
  (params (AxisValue :type "Float (single-precision)")))

(event `ServerMoveVertical`
  (params (Delta :type "Vector Structure"))
  (`self.MulticastMoveVertical` Delta))

(event `MulticastMoveVertical`
  (params (Delta :type "Vector Structure"))
  (bind _asbp_platform_pawn (cast `/Game/PingPong/Blueprints/BP_PlatformPawn` (`self.K2_GetPawn`)))
  (`/Game/PingPong/Blueprints/BP_PlatformPawn.MoveVertical` _asbp_platform_pawn Delta))

(event `InputAction|RespawnBall`
  (params (Key :type "Key Structure"))
  (:`Pressed`
    (`self.Server RespawnBall`)))

(event `Server RespawnBall`
  (bind _asbp_ping_pong_game_mode_base (cast `/Game/PingPong/Blueprints/BP_PingPongGameModeBase` (`GameplayStatics.GetGameMode`)))
  (`self.K2_DestroyActor` (`PingPongGameModeBase.Ball` _asbp_ping_pong_game_mode_base)))

(fn `UserConstructionScript`)