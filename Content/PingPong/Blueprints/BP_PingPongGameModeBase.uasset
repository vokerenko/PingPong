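; Game mode for a two-player Pong match that waits for both players before putting the ball in play.
; PostLogin stores each player controller and counts joins, while Tick prints a waiting message during solo presence.
; When the second player joins, it spawns the ball after a short delay and sets the Pong HUD on each client.
; The ball's OnDestroyed event drives a delayed respawn, rebinding on each new ball to keep play going.
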(event `self.ReceiveBeginPlay`)

(event `self.ReceiveTick`
  (params (DeltaSeconds :type "Float (single-precision)"))
  (if (== (`self.NumberOfPlayers`) 1)
    (`KismetSystemLibrary.PrintString` "Waiting for a second player to join" true true (struct :`G` 0.66 :`B` 1.0 :`A` 1.0) 0.0)))

(event `self.K2_PostLogin`
  (params (NewPlayer :type "PlayerController Object Reference"))
  (bind _numberofplayers (`self.NumberOfPlayers`))
  (bind _asbp_player_controller (cast `/Game/PingPong/Blueprints/BP_PlayerController` NewPlayer))
  (`KismetArrayLibrary.Array_Add` (`self.Players`) _asbp_player_controller)
  (bind _result (`/Engine/EditorBlueprintResources/StandardMacros.IncrementInt` (`self.NumberOfPlayers`))
    (:`  `
      (bind _output_get (set `self.NumberOfPlayers` _result))
      (`KismetSystemLibrary.PrintString` (`KismetStringLibrary.Concat_StrStr` "The player " (`KismetStringLibrary.Conv_IntToString` _output_get) " has joined the game") true true (struct :`G` 0.66 :`B` 1.0 :`A` 1.0) 6.0)
      (if (== _numberofplayers 1)
        _
        (elif (== _numberofplayers 2)
          (`KismetSystemLibrary.Delay` 1.0)
          (bind _returnvalue (`|SpawnActorFromClass` "/Game/PingPong/Blueprints/BP_Ball.BP_Ball_C" (`KismetMathLibrary.MakeTransform` (30.0 -170.0 -30.0)) "Undefined" "OverrideRootScale" null null))
          (bind _output_get_2 (set `self.Ball` _returnvalue))
          (add `Actor.OnDestroyed` _output_get_2 (delegate `RespawnNewBall`))
          (for (_array_element _array_index) (`self.Players`)
            (`PlayerController.ClientSetHUD` _array_element "/Game/PingPong/Blueprints/BP_PongHUD.BP_PongHUD_C")))))))

(event `RespawnNewBall`
  (params (DestroyedActor :type "Actor Object Reference"))
  (clear `Actor.OnDestroyed` DestroyedActor)
  (`KismetSystemLibrary.Delay` 1.0)
  (bind _returnvalue (`|SpawnActorFromClass` "/Game/PingPong/Blueprints/BP_Ball.BP_Ball_C" (`KismetMathLibrary.MakeTransform` (30.0 -170.0 -30.0)) "Undefined" "OverrideRootScale" null null))
  (bind _output_get (set `self.Ball` _returnvalue))
  (add `Actor.OnDestroyed` _output_get (delegate `RespawnNewBall`)))

(fn `UserConstructionScript`)