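; Ping-pong ball actor that awards a point and destroys itself when it overlaps an actor tagged Player or Enemy.
; The construction script gives its ProjectileMovement a random diagonal velocity on the XY plane.
; On overlap it gathers all BP_PlatformPawn actors and increments Score on the first for Player or the second for Enemy, so scoring depends on the array order.
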(event `self.ReceiveBeginPlay`)

(event `self.ReceiveActorBeginOverlap`
  (params (OtherActor :type "Actor Object Reference"))
  (bind _outactors (`GameplayStatics.GetAllActorsOfClass` "/Game/PingPong/Blueprints/BP_PlatformPawn.BP_PlatformPawn_C"))
  (for (_array_element _array_index) _outactors
    (if (`self.ActorHasTag` OtherActor "Player")
      (if (== _array_index 0)
        (bind _result (`/Engine/EditorBlueprintResources/StandardMacros.IncrementInt` (`/Game/PingPong/Blueprints/BP_PlatformPawn.Score` _array_element))
          (:`  `
            (set `/Game/PingPong/Blueprints/BP_PlatformPawn.Score` _result _array_element)
            (`self.K2_DestroyActor` :!label _label))))
      (elif (`self.ActorHasTag` OtherActor "Enemy")
        (if (== _array_index 1)
          (bind _result_2 (`/Engine/EditorBlueprintResources/StandardMacros.IncrementInt` (`/Game/PingPong/Blueprints/BP_PlatformPawn.Score` _array_element))
            (:`  `
              (set `/Game/PingPong/Blueprints/BP_PlatformPawn.Score` _result_2 _array_element)
              (goto _label))))))))

(event `self.ReceiveTick`
  (params (DeltaSeconds :type "Float (single-precision)")))

(fn `UserConstructionScript`
  (set `MovementComponent.Velocity` (`KismetMathLibrary.MakeVector` (select `bool` (`KismetMathLibrary.RandomBool`) :`false` -1.0 :`true` 1.0 :!type "Float (single-precision)") (select `bool` (`KismetMathLibrary.RandomBool`) :`false` -1.0 :`true` 1.0 :!type "Float (single-precision)")) (`self.ProjectileMovement`)))