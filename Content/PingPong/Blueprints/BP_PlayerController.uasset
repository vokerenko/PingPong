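; Player controller for the PingPong game that drives the player's possessed BP_PlatformPawn from the MoveVertical axis input.
; Input scales the pawn's right vector by axis value and Speed, then passes that delta to ServerMoveVertical.
; With authority, it relays the delta through MulticastMoveVertical, which calls MoveVertical on the controlled pawn.
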(event `InputAxis|MoveVertical`
  (params (AxisValue :type "Float (single-precision)"))
  (bind _asbp_platform_pawn (cast `/Game/PingPong/Blueprints/BP_PlatformPawn` (`self.K2_GetPawn`)))
  (`self.ServerMoveVertical` (* (* (`self.GetActorRightVector` _asbp_platform_pawn) AxisValue) (`/Game/PingPong/Blueprints/BP_PlatformPawn.Speed` _asbp_platform_pawn))))

(event `ServerMoveVertical`
  (params (Delta :type "Vector Structure"))
  (`/Engine/EditorBlueprintResources/ActorMacros.Switch Has Authority`
    (:`Authority`
      (`self.MulticastMoveVertical` Delta))))

(event `MulticastMoveVertical`
  (params (Delta :type "Vector Structure"))
  (bind _asbp_platform_pawn (cast `/Game/PingPong/Blueprints/BP_PlatformPawn` (`self.K2_GetPawn`)))
  (`/Game/PingPong/Blueprints/BP_PlatformPawn.MoveVertical` _asbp_platform_pawn Delta))

(fn `UserConstructionScript`)